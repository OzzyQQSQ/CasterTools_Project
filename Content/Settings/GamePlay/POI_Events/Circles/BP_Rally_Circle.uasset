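; BP_Rally_Circle is a decal actor that shows a rally point radius, colored by team.
; On BeginPlay it creates a dynamic instance of the radius decal material and sets its Color parameter from the HUD color set, choosing the Team or Enemy tint by the rally's team ID.
; On Tick it destroys itself once the referenced Rally is no longer valid.
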(event `self.ReceiveBeginPlay`
  (bind _rallydecal (`self.RallyDecal`))
  (`DecalComponent.SetDecalMaterial` _rallydecal "/CasterTools_Project/Settings/GamePlay/POI_Events/Circles/M_Rally_Radius_Inst.M_Rally_Radius_Inst")
  (bind _returnvalue (`DecalComponent.CreateDynamicMaterialInstance` _rallydecal))
  (set `self.RallyMaterial` _returnvalue)
  (bind _returnvalue_2 (message `SQTeamInterface.GetTeamId` (`self.Rally`)))
  (`MaterialInstanceDynamic.SetVectorParameterValue` (`self.RallyMaterial`) "Color" (`SQColorsDataAsset.GetColor` (`/Game/UI/Library_SquadUI.Get SQHUD Colors`) (select `bool` (== _returnvalue_2 (`self.Team`)) :`false` "Enemy" :`true` "Team" :!type "ESQMapWidgetTint Enum") -1)))

(event `self.ReceiveTick`
  (params (DeltaSeconds :type "Float (single-precision)"))
  (`self.Rally`
    (:`then`)
    (:`else`
      (`self.K2_DestroyActor`))))

(fn `UserConstructionScript`)