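; Decal actor that draws a circle for a HAB, colored by that HAB's current state.
; On BeginPlay it applies a siege-circle material to its decal and creates a dynamic instance of it.
; Each Tick polls the linked HAB, setting the color to orange while unbuilt, red when its spawn point is sieged, and white otherwise.
; The actor destroys itself when the HAB reference is no longer valid.
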(event `self.ReceiveBeginPlay`
  (bind _habdecal (`self.HabDecal`))
  (`DecalComponent.SetDecalMaterial` _habdecal "/CasterTools_Project/Settings/GamePlay/POI_Events/Textures/Cast_MI_CircleSiege_Inst.Cast_MI_CircleSiege_Inst")
  (bind _returnvalue (`DecalComponent.CreateDynamicMaterialInstance` _habdecal))
  (set `self.Material` _returnvalue))

(event `self.ReceiveTick`
  (params (DeltaSeconds :type "Float (single-precision)"))
  (bind _hab_v (`self.Hab_v`)
    (:`then`
      (if (`|EnumInequality` (`SQDeployable.BuildState` _hab_v) "Completed")
        (`MaterialInstanceDynamic.SetVectorParameterValue` (`self.Material`) "Color" (struct :`R` 0.938686 :`G` 0.552011 :`A` 1.0))
        (elif (`SQGameSpawn.GetSieged` (`/Game/Gameplay/Deployables/BP_Deployable_Hab.MySpawnPoint` _hab_v))
          (`MaterialInstanceDynamic.SetVectorParameterValue` (`self.Material`) "Color" (struct :`R` 1.0 :`A` 1.0))
          (else
            (`MaterialInstanceDynamic.SetVectorParameterValue` (`self.Material`) "Color" (struct :`R` 1.0 :`G` 1.0 :`B` 1.0 :`A` 1.0))))))
    (:`else`
      (`self.K2_DestroyActor`))))

(fn `UserConstructionScript`)