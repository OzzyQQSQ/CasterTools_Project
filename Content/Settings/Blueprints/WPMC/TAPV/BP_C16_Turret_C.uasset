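; Turret Blueprint for the TAPV's C16 weapon in Squad, handling fire input, camera zoom and turret aiming.
; Fire input starts and stops the vehicle inventory's current weapon, while a timeline eases first-person FOV to the user's FOV divided by the zoom level.
; Construction binds TurretMovement to yaw and pitch components and registers it; getters expose attach points.
; Rotation audio setup is disconnected pending a stabilised-turret revisit (SQ-8134).
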(event `InputAction|Fire`
  (params (Key :type "Key Structure"))
  (bind _currentweapon (`SQPawnInventoryComponent.CurrentWeapon` (`self.GetVehicleInventory`)))
  (:`Pressed`
    (`SQEquipableItem.BeginUse` _currentweapon))
  (:`Released`
    (`SQEquipableItem.EndUse` _currentweapon)))

(event `self.ReceiveBeginPlay`
  ;[1 1 1] BeginPlay
  (`ActorComponent.SetActive` (`self.FirstPersonCamera`) true false)
  (`self.ResetZoom`))

(event `self.BP_OnVehicleZoom`
  (bind _firstpersoncamera (`self.FirstPersonCamera`))
  ;[0 0.685 0.1713] ZoomEvents
  (bind (_direction _lerp) (`Timeline|Timeline_0` :!via `PlayFromStart`)
    (:`Update`
      (`CameraComponent.SetFieldOfView` _firstpersoncamera (`KismetMathLibrary.Lerp` (`CameraComponent.FieldOfView` _firstpersoncamera) (/ (`SQGameUserSettings.FOV` (`SQBlueprintLibrary.GetSquadGameUserSettings`)) (`|GetArrayItem` (`self.ZoomLevels`) (`self.CurrentZoom`))) _lerp)))))

(event `self.ResetZoom`
  ;[0 0.685 0.1713] ZoomEvents
  (`CameraComponent.SetFieldOfView` (`self.FirstPersonCamera`) (/ (`SQGameUserSettings.FOV` (`SQBlueprintLibrary.GetSquadGameUserSettings`)) (`|GetArrayItem` (`self.ZoomLevels`))))
  (`CameraComponent.SetFieldOfView` (`self.Camera`) (/ (`SQGameUserSettings.FOV` (`SQBlueprintLibrary.GetSquadGameUserSettings`)) (`|GetArrayItem` (`self.ZoomLevels`))))
  (`ActorComponent.SetActive` (`self.Camera`) false false)
  (`ActorComponent.SetActive` (`self.FirstPersonCamera`) true false)
  (set `self.CurrentZoom` 0))

(fn `Get1PAttachComponent`
  (returns (ReturnValue :type "SceneComponent Object Reference"))
  (return (`self.GunAttachPoint`)))

(fn `Get3PAttachComponent`
  (returns (ReturnValue :type "SceneComponent Object Reference"))
  (return (`self.GunAttachPoint`)))

(fn `GetMasterPoseComponent`
  (returns (ReturnValue :type "SkinnedMeshComponent Object Reference"))
  (return null))

(fn `GetSoldierAttachComponent`
  (returns (ReturnValue :type "SceneComponent Object Reference"))
  (return (`SQVehicle.VehicleMesh` (`self.GetVehicle`))))

(fn `GetTurretMovementComponent`
  (returns (ReturnValue :type "SQTurretMovementComponent Object Reference"))
  (return (`self.TurretMovement`)))

(fn `GetWeaponAttachComponent`
  (returns (ReturnValue :type "SceneComponent Object Reference"))
  (return (`self.GunAttachPoint`)))

(fn `UserConstructionScript`
  (bind _turretmovement (`self.TurretMovement`))
  (`|ExecutionSequence`
    (:`then_0`
      (set `SQTurretMovementComponent.UpdatedPitchComponent` (`self.GunAttachPoint`) _turretmovement)
      (set `SQTurretMovementComponent.UpdatedYawComponent` (`self.Scene`) _turretmovement)
      (set `SQVelocityRotatingMovementComponent.HeadingParentComponent` _turretmovement _turretmovement)
      (`SQMovementComponentManager.RegisterComponent` (`self.MovementComponentManager`) _turretmovement))))