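; Caster camera pawn that gives a broadcaster a HUD, target highlighting and a picture-in-picture view of a spectated soldier.
; On locally controlled clients, Tick sphere-traces from the camera and highlights the hit soldier or vehicle through custom depth stencil.
; AttachSpectateCam reuses or spawns a scene-capture camera, attaches it to a soldier mesh socket and shows its HUD panel.
; Transparent mode is delegated to the caster player controller.
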(event `self.ReceiveBeginPlay`
  (bind _returnvalue (`GameplayStatics.GetPlayerController` 0))
  (`parent.ReceiveBeginPlay`)
  (`|ExecutionSequence`
    (:`then_0`
      (if (== (`Controller.K2_GetPawn` _returnvalue) self)
        (bind _caster_ui (`self.Caster_UI`)
          (:`then`
            (`Widget.SetVisibility` _caster_ui "Hidden"))
          (:`else`
            (bind _returnvalue_2 (`|CreateWidget` "/CasterTools_Project/Settings/UI/CasterOverlay/W_Caster_HUD.W_Caster_HUD_C" _returnvalue))
            (bind _output_get (set `self.Caster_UI` _returnvalue_2))
            (`/Engine/EditorBlueprintResources/StandardMacros.IsValid` _output_get
              (:`Is Valid`
                (`UserWidget.AddToViewport` _output_get 0)))))))))

(event `self.ReceiveTick`
  (params (DeltaSeconds :type "Float (single-precision)"))
  (`parent.ReceiveTick` 0.0)
  (`/Engine/EditorBlueprintResources/ActorMacros.Switch Has Authority`
    (:`Remote`
      (if (`self.IsLocallyControlled`)
        (`self.ActorSpherePick`)))))

(event `Transparent_Mode`
  ;[1 0.3719 0.4317 0.253] Transparent Mod
  (`/CasterTools_Project/Settings/Core/Caster_PlayerController_Child.Execute Transparent` (cast `/CasterTools_Project/Settings/Core/Caster_PlayerController_Child` (`SQGameplayService.TryGetLocalPlayerController`) :!pure true)))

(event `self.ReceiveEndPlay`
  (params (EndPlayReason :type "EEndPlayReason Enum" :default "Destroyed"))
  ;[0 0 0 0.415] EventEndPlay
  (`parent.ReceiveEndPlay` EndPlayReason)
  (bind _caster_ui (`self.Caster_UI`)
    (:`then`
      (`Widget.SetVisibility` _caster_ui "Hidden")
      (`/CasterTools_Project/Settings/Core/Caster_PlayerController_Child.Transparent Off` (cast `/CasterTools_Project/Settings/Core/Caster_PlayerController_Child` (`SQGameplayService.TryGetLocalPlayerController`) :!pure true)))
    (:`else`)))

(fn `ActorSpherePick`
  (bind _firstpersoncameracomponent (`self.FirstPersonCameraComponent`))
  (bind _current_target_actor (`self.Current Target Actor`))
  (bind _current_target_actor_2 (`self.Current Target Actor`))
  (bind _returnvalue (`SceneComponent.K2_GetComponentLocation` _firstpersoncameracomponent))
  (bind _returnvalue_2 (`KismetMathLibrary.Conv_RotatorToVector` (`SceneComponent.K2_GetComponentRotation` _firstpersoncameracomponent)))
  (bind _outhit (`KismetSystemLibrary.SphereTraceSingleForObjects` :`Start` (+ _returnvalue (* _returnvalue_2 (`KismetMathLibrary.Conv_DoubleToVector` 200.0))) :`End` (+ _returnvalue (* _returnvalue_2 (`KismetMathLibrary.Conv_DoubleToVector` (`self.Target Attachment Trace Dist`)))) :`ObjectTypes` (`|MakeArray` "ObjectTypeQuery3" "ObjectTypeQuery5" :!type "EObjectTypeQuery Enum") :`DrawDebugType` "Persistent" :`TraceColor` (struct :`R` 0.074214 :`G` 0.630757 :`B` 0.822786 :`A` 1.0)))
  (if (`KismetSystemLibrary.IsValid` (`.HitActor` (`GameplayStatics.BreakHitResult` _outhit)))
    (if (and (== _current_target_actor (`.HitActor` (`GameplayStatics.BreakHitResult` _outhit))) (`KismetSystemLibrary.IsValid` _current_target_actor))
      (`self.UpdateStensil`)
      (else
        (bind _output_get (set `self.Current Target Actor` (`.HitActor` (`GameplayStatics.BreakHitResult` _outhit))))
        (if (`KismetMathLibrary.ClassIsChildOf` (`GameplayStatics.GetObjectClass` _output_get) "/Script/Squad.SQSoldier")
          (bind _asbp_mutable_soldier (cast `/Game/Blueprints/Soldiers/BP_MutableSoldier` _current_target_actor_2))
          (bind (_assqsoldier _bsuccess) (cast `SQSoldier` (`.HitActor` (`GameplayStatics.BreakHitResult` _outhit)) :!pure true))
          (if (or (and (not (`SQSoldier.bIsDying` _assqsoldier)) (not (`SQSoldier.bIsWounded` _assqsoldier)) (not (`Actor.bHidden` _assqsoldier))) (not _bsuccess))
            (bind _output_get_2 (set `self.As BP Mutable Soldier` _asbp_mutable_soldier))
            (`PrimitiveComponent.SetCustomDepthStencilValue` (`Character.Mesh` _output_get_2) 252))
          (else
            (bind _assqvehicle (cast `SQVehicle` _current_target_actor_2))
            (bind _output_get_3 (set `self.As SQVehicle` _assqvehicle))
            (bind _vehiclemesh (`SQVehicle.VehicleMesh` _output_get_3))
            (`PrimitiveComponent.SetRenderCustomDepth` _vehiclemesh true)
            (`PrimitiveComponent.SetCustomDepthStencilValue` _vehiclemesh 252)))))
    (else
      (`self.Current Target Actor`
        (:`then`
          (set `self.Current Target Actor` null)
          (bind _as_sqvehicle (`self.As SQVehicle`)
            (:`then`
              (`PrimitiveComponent.SetRenderCustomDepth` (`SQVehicle.VehicleMesh` _as_sqvehicle) false))
            (:`else`)))
        (:`else`)))))

(fn `AttachSpectateCam`
  (bind _currentspectatecam (`self.CurrentSpectateCam`))
  (bind _springarm (`/CasterTools_Project/Settings/GamePlay/SpectateCam/BP_SpectateCam_Caster.SpringArm` (`self.CurrentSpectateCam`)))
  (`/Engine/EditorBlueprintResources/StandardMacros.IsValid` _currentspectatecam
    (:`Is Valid`
      (`KismetArrayLibrary.Array_Clear` (`SceneCaptureComponent.HiddenActors` (`/CasterTools_Project/Settings/GamePlay/SpectateCam/BP_SpectateCam_Caster.SceneCaptureComponent2D` _currentspectatecam))))
    (:`Is Not Valid`
      (bind _returnvalue (`|SpawnActorFromClass` "/CasterTools_Project/Settings/GamePlay/SpectateCam/BP_SpectateCam_Caster.BP_SpectateCam_Caster_C" (`KismetMathLibrary.MakeTransform` (0.0 0.0 0.0)) "AlwaysSpawn" "OverrideRootScale" null self))
      (bind _output_get (set `self.CurrentSpectateCam` _returnvalue))))
  (`KismetArrayLibrary.Array_Add` (`SceneCaptureComponent.HiddenActors` (`/CasterTools_Project/Settings/GamePlay/SpectateCam/BP_SpectateCam_Caster.SceneCaptureComponent2D` _output_get)) (`self.CurrentSpectSoldier`))
  (`SceneComponent.K2_AttachToComponent` _springarm (`Character.Mesh` (`self.CurrentSpectSoldier`)) (`self.CurrentInsertCamSocketN`) "SnapToTarget" "SnapToTarget" "KeepRelative" true)
  (`SceneComponent.K2_AddLocalOffset` _springarm (`KismetMathLibrary.MakeVector` (`self.SpectateInsertCam Forward_O`) (`self.SpectateInsertCam Height_O`) (`self.SpectateInsertCam Right_O`)) false false)
  (`self.K2_SetActorRelativeRotation` (`KismetMathLibrary.MakeRotator` 0.0 (`self.SpectateInsertCam Pitch_O`) (`self.SpectateInsertCam Yaw_O`)))
  (`/CasterTools_Project/Settings/UI/CasterOverlay/W_Caster_HUD.SetSpectatorCamVisibility` (cast `/CasterTools_Project/Settings/UI/CasterOverlay/W_Caster_HUD` (`self.Caster_UI`) :!pure true) true))

(fn `DetachSpectateCam`
  (bind _currentspectsoldier (`self.CurrentSpectSoldier`))
  (`/Engine/EditorBlueprintResources/StandardMacros.IsValid` _currentspectsoldier
    (:`Is Valid`
      (`self.K2_DetachFromActor` _currentspectsoldier "KeepWorld" "KeepWorld" "KeepRelative"))
    (:`Is Not Valid`
      _))
  (`self.K2_DestroyActor` _currentspectsoldier)
  (`/CasterTools_Project/Settings/UI/CasterOverlay/W_Caster_HUD.SetSpectatorCamVisibility` (cast `/CasterTools_Project/Settings/UI/CasterOverlay/W_Caster_HUD` (`self.Caster_UI`) :!pure true) false))

(fn `GetSpectatedSoldierFullName`
  (returns (NewParam :type String))
  (bind _assqplayer_state (cast `SQPlayerState` (`Pawn.PlayerState` (`self.CurrentSpectSoldier`)))
    (:`then`
      (return (`SQPlayerState.GetFullPlayerName` _assqplayer_state false)))
    (:`CastFailed`
      (return (`self.FallbackSpectatedPlayerFullName`)))))

(fn `UpdateStensil`
  (`|ExecutionSequence`
    (:`then_0`
      (bind _as_bp_mutable_soldier (`self.As BP Mutable Soldier`)
        (:`then`
          (`PrimitiveComponent.SetCustomDepthStencilValue` (`Character.Mesh` _as_bp_mutable_soldier) 252))
        (:`else`)))
    (:`then_1`
      (bind _as_sqvehicle (`self.As SQVehicle`)
        (:`then`
          (`PrimitiveComponent.SetCustomDepthStencilValue` (`SQVehicle.VehicleMesh` _as_sqvehicle) 252))
        (:`else`)))))

(fn `UserConstructionScript`
  (`parent.UserConstructionScript`))