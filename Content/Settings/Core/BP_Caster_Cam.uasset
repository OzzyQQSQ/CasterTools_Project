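; Caster/spectator camera pawn that shows a caster HUD, follows soldiers and vehicles, and toggles radius circles on HABs and squad rallies.
; A per-tick sphere trace picks the aimed target and outlines it via custom depth stencil.
; That target feeds a spawned POV camera with status widgets, or a zoomable follow cam that detaches on death, wounding or destruction.
; It also teleports via map position.
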(event `self.ReceiveBeginPlay`
  (bind _returnvalue (`GameplayStatics.GetPlayerController` 0))
  (`parent.ReceiveBeginPlay`)
  (`|ExecutionSequence`
    (:`then_0`
      (if (== (`Controller.K2_GetPawn` _returnvalue) self)
        (bind _caster_ui (`self.Caster_UI`)
          (:`then`
            (`Widget.SetVisibility` _caster_ui "Visible"))
          (:`else`
            (bind _returnvalue_2 (`|CreateWidget` "/CasterTools_Project/Settings/UI/CasterOverlay/W_Caster_HUD.W_Caster_HUD_C" _returnvalue))
            (bind _output_get (set `self.Caster_UI` _returnvalue_2))
            (`/Engine/EditorBlueprintResources/StandardMacros.IsValid` _output_get
              (:`Is Valid`
                (set `self.SpectatorCamWidget` (`/CasterTools_Project/Settings/UI/CasterOverlay/W_Caster_HUD.W_SpecCam_Caster` _returnvalue_2))
                (set `self.W Follow Name` (`/CasterTools_Project/Settings/UI/CasterOverlay/W_Caster_HUD.W_FollowName` _returnvalue_2))
                (set `self.W Infantry Status Caster` (`/CasterTools_Project/Settings/UI/CasterOverlay/W_Caster_HUD.W_InfantryStatusCaster` _returnvalue_2))
                (set `self.W Vehicle Status Caster` (`/CasterTools_Project/Settings/UI/CasterOverlay/W_Caster_HUD.W_VehicleStatusCaster` _returnvalue_2))
                (`UserWidget.AddToViewport` _output_get 0)))))))))

(event `self.ReceiveTick`
  (params (DeltaSeconds :type "Float (single-precision)"))
  ;[0 0 0 0.546] Tick Events
  (`parent.ReceiveTick` 0.0)
  (if (`self.IsLocallyControlled` (`GameplayStatics.GetPlayerPawn` 0))
    (`self.ActorSpherePick`)))

(event `Key|MouseScrollDown`
  (params (Key :type "Key Structure"))
  ;[0.05616 0.3343 1 0.253] Keybinds
  ;;[1 1 1] FollowCam
  (:`Released`
    (if (`self.bIsFollowingActor`)
      (`self.Increase SpringArm`))))

(event `Key|MouseScrollUp`
  (params (Key :type "Key Structure"))
  ;[0.05616 0.3343 1 0.253] Keybinds
  ;;[1 1 1] FollowCam
  (:`Released`
    (if (`self.bIsFollowingActor`)
      (`self.Decrease SpringArm`))))

(event `Transparent_Mode`
  ;[1 0.3719 0.4317 0.253] Transparent Mod
  (`/CasterTools_Project/Settings/Core/Caster_PlayerController_Child.Execute Transparent` (cast `/CasterTools_Project/Settings/Core/Caster_PlayerController_Child` (`SQGameplayService.TryGetLocalPlayerController`) :!pure true)))

(event `Key|H`
  (params (Key :type "Key Structure"))
  ;[0.05616 0.3343 1 0.253] Keybinds
  ;;[1 1 1] Hab Circle
  (:`Released`
    (`self.Hab Radius`)))

(event `Key|P`
  (params (Key :type "Key Structure"))
  ;[0.05616 0.3343 1 0.253] Keybinds
  ;;[1 1 1] Rally Circle
  (:`Released`
    (`self.Rally Radius`)))

(event `self.ReceiveEndPlay`
  (params (EndPlayReason :type "EEndPlayReason Enum" :default "Destroyed"))
  ;[0 0 0 0.415] EventEndPlay
  (`parent.ReceiveEndPlay` EndPlayReason)
  (bind _caster_ui (`self.Caster_UI`)
    (:`then`
      (`Widget.SetVisibility` _caster_ui "Hidden")
      (`/CasterTools_Project/Settings/Core/Caster_PlayerController_Child.Transparent Off` (cast `/CasterTools_Project/Settings/Core/Caster_PlayerController_Child` (`SQGameplayService.TryGetLocalPlayerController`) :!pure true)))
    (:`else`)))

(event `Attach SpecCam`
  ;[0.436 1 0.3404 0.133] POV Cam
  (`self.SpawnSpectatorCam`)
  (`self.Current Target Actor`
    (:`then`
      (`self.Dettach POV Cam`)
      (`self.Attach POV Cam`))
    (:`else`)))

(event `SpawnSpectatorCam`
  (bind (_returnvalue_location _returnvalue_rotation) (`KismetMathLibrary.BreakTransform` (`self.GetTransform` self)))
  ;[0.436 1 0.3404 0.133] POV Cam
  (bind _outactors (`GameplayStatics.GetAllActorsOfClass` "/CasterTools_Project/Settings/GamePlay/SpectateCam/BP_SpectateCam_Caster_M.BP_SpectateCam_Caster_M_C"))
  (if (== (`KismetArrayLibrary.Array_Length` _outactors) 0)
    (if (`self.IsLocallyControlled`)
      (`/Engine/EditorBlueprintResources/StandardMacros.IsValid` (`self.CameraPlayer`)
        (:`Is Not Valid`
          (bind _returnvalue (`|SpawnActorFromClass` "/CasterTools_Project/Settings/GamePlay/SpectateCam/BP_SpectateCam_Caster_M.BP_SpectateCam_Caster_M_C" (`KismetMathLibrary.MakeTransform` _returnvalue_location _returnvalue_rotation) "AlwaysSpawn" "OverrideRootScale" self null))
          (set `self.CameraPlayer` _returnvalue))))
    (else
      (set `self.CameraPlayer` (`|GetArrayItem` _outactors)))))

(event `Attach FollowCam`
  (params (Actor :type "Actor Object Reference") (SM :type "SceneComponent Object Reference"))
  ;[1 0.02604 0.02604 0.065] FollowCam
  (`CharacterMovementComponent.DisableMovement` (`self.CharacterMovement`))
  (`self.K2_AttachToComponent` SM "None" "SnapToTarget" "KeepRelative" "KeepRelative")
  (`SceneComponent.SetAbsolute` (`self.CapsuleComponent`) false true true)
  (`self.PostFollowCamAttached_Client`))

(event `FollowCam`
  ;[1 0.02604 0.02604 0.065] FollowCam
  (if (`self.bIsFollowingActor`)
    (if (`KismetSystemLibrary.IsValid` (`self.Current Target Actor`))
      (`self.Enter Follow Cam` :!label _label)
      (else
        (`self.ExitFollowCam`)))
    (else
      (goto _label))))

(event `PostFollowCamDettached`
  (bind _springarm (`self.SpringArm`))
  ;[1 0.02604 0.02604 0.065] FollowCam
  (set `SpringArmComponent.TargetOffset` (0.0 0.0 0.0) _springarm)
  (set `SpringArmComponent.TargetArmLength` 0.0 _springarm)
  (set `self.bIsFollowingActor` false))

(event `OnFollowSoldierDeath`
  ;[1 0.02604 0.02604 0.065] FollowCam
  (`self.ExitFollowCam` :!label _label_2))

(event `OnFollowVehicleDestroyed`
  (params (Vehicle :type "SQVehicle Object Reference"))
  ;[1 0.02604 0.02604 0.065] FollowCam
  (goto _label_2))

(event `OnFollowTargetEndPlay`
  (params (Actor :type "Actor Object Reference") (EndPlayReason :type "EEndPlayReason Enum" :default "Destroyed"))
  ;[1 0.02604 0.02604 0.065] FollowCam
  (goto _label_2))

(event `PostFollowCamAttached_Client`
  ;[1 0.02604 0.02604 0.065] FollowCam
  (set `SpringArmComponent.TargetOffset` (0.0 0.0 300.0) (`self.SpringArm`))
  (set `SpringArmComponent.TargetArmLength` 1500.0 (`self.SpringArm`))
  (set `self.bIsFollowingActor` true))

(event `OnFollowTargetDestroyed`
  (params (DestroyedActor :type "Actor Object Reference"))
  ;[1 0.02604 0.02604 0.065] FollowCam
  (goto _label_2))

(event `OnFollowedPlayerWounded`
  ;[1 0.02604 0.02604 0.065] FollowCam
  (goto _label_2))

(event `DetachAdminCamFromActor`
  (params (`Movement Mode` :type "EMovementMode Enum" :default "MOVE_None"))
  ;[1 0.02604 0.02604 0.065] FollowCam
  (`self.K2_DetachFromActor` "KeepWorld")
  (`CharacterMovementComponent.SetMovementMode` (`self.CharacterMovement`) `Movement Mode` 0)
  (`self.PostFollowCamDettached`))

(event `Increase SpringArm`
  (bind _springarm (`self.SpringArm`))
  ;[1 0.02604 0.02604 0.065] FollowCam
  (set `SpringArmComponent.TargetArmLength` (+ (`SpringArmComponent.TargetArmLength` _springarm) 50.0) _springarm))

(event `Decrease SpringArm`
  (bind _springarm (`self.SpringArm`))
  ;[1 0.02604 0.02604 0.065] FollowCam
  (set `SpringArmComponent.TargetArmLength` (+ (`SpringArmComponent.TargetArmLength` _springarm) -50.0) _springarm))

(event `Teleport`
  (bind _mapcore (`/Game/UI/BP_HUD.MapCore` (cast `/Game/UI/BP_HUD` (`PlayerController.GetHUD` (`GameplayStatics.GetPlayerController` 0)) :!pure true)))
  ;[0 0 0 0.54] Teleport
  (if (`Widget.IsHovered` _mapcore)
    (`self.TeleportServer` (.x (`/Game/UI/BPFL_MapConversions.Mouse Position to World Location` (`KismetInputLibrary.PointerEvent_GetScreenSpacePosition` (`/Game/UI/Widgets/Map/W_SQMapCore.Mouse Move Event` _mapcore)))) (.y (`/Game/UI/BPFL_MapConversions.Mouse Position to World Location` (`KismetInputLibrary.PointerEvent_GetScreenSpacePosition` (`/Game/UI/Widgets/Map/W_SQMapCore.Mouse Move Event` _mapcore)))) (.z (`SceneComponent.K2_GetComponentLocation` (`self.CapsuleComponent`))))))

(event `TeleportServer`
  (params (`New Location X` :type "Float (double-precision)") (`New Location Y` :type "Float (double-precision)") (`New Location Z` :type "Float (double-precision)"))
  ;[0 0 0 0.54] Teleport
  (`self.K2_SetActorLocation` (`KismetMathLibrary.MakeVector` `New Location X` `New Location Y` `New Location Z`) false true))

(event `Hab Radius`
  (bind _timerhandlehab (`self.TimerHandleHab`))
  (bind _habcirclearray (`self.HabCircleArray`))
  ;[0.09549 0.2229 1 0.264] POI Hab/Rally
  ;;[1 1 1 0.193] Hab Circle
  (`/Engine/EditorBlueprintResources/StandardMacros.FlipFlop`
    (:`A`
      (if (`KismetSystemLibrary.K2_IsValidTimerHandle` _timerhandlehab)
        (`KismetSystemLibrary.K2_UnPauseTimerHandle` _timerhandlehab)
        (else
          (bind _returnvalue (`KismetSystemLibrary.K2_SetTimerDelegate` (delegate `Update Habs`) 0.1 true))
          (set `self.TimerHandleHab` _returnvalue))))
    (:`B`
      (`KismetSystemLibrary.K2_PauseTimerHandle` _timerhandlehab)
      (for _array_element _habcirclearray
        (`self.K2_DestroyActor` _array_element))
      (`KismetArrayLibrary.Array_Clear` _habcirclearray)
      (`KismetArrayLibrary.Array_Clear` _habcirclearray))))

(event `Update Habs`
  ;[0.09549 0.2229 1 0.264] POI Hab/Rally
  ;;[1 1 1 0.193] Hab Circle
  (bind _outactors (`GameplayStatics.GetAllActorsOfClass` "/Game/Gameplay/Deployables/BP_Deployable_Hab.BP_Deployable_Hab_C"))
  (for _array_element _outactors
    (bind _returnvalue (`KismetArrayLibrary.Array_AddUnique` (`self.HabArray`) _array_element))
    (if (!= _returnvalue -1)
      (bind _returnvalue_2 (`|SpawnActorFromClass` "/CasterTools_Project/Settings/GamePlay/POI_Events/Circles/BP_Hab_Circle.BP_Hab_Circle_C" (`KismetMathLibrary.MakeTransform` (`SceneComponent.K2_GetComponentLocation` (`Actor.RootComponent` (`|GetArrayItem` (`self.HabArray`) _returnvalue)))) "Undefined" "OverrideRootScale" null _array_element null))
      (`KismetArrayLibrary.Array_Add` (`self.HabCircleArray`) _returnvalue_2))))

(event `Rally Radius`
  (bind _rally_circle_array (`self.Rally Circle Array`))
  (bind _timerhandlerally (`self.TimerHandleRally`))
  ;[0.09549 0.2229 1 0.264] POI Hab/Rally
  ;;[1 1 1 0.081] Rally Circle
  (`/Engine/EditorBlueprintResources/StandardMacros.FlipFlop`
    (:`A`
      (if (`KismetSystemLibrary.K2_IsValidTimerHandle` _timerhandlerally)
        (`KismetSystemLibrary.K2_UnPauseTimerHandle` _timerhandlerally)
        (else
          (bind _returnvalue (`KismetSystemLibrary.K2_SetTimerDelegate` (delegate `UpdateRally`) 0.1 true))
          (set `self.TimerHandleRally` _returnvalue))))
    (:`B`
      (`KismetSystemLibrary.K2_PauseTimerHandle` _timerhandlerally)
      (for _array_element (`self.Rally Array`)
        (`self.K2_DestroyActor` _array_element))
      (`KismetArrayLibrary.Array_Clear` _rally_circle_array)
      (`KismetArrayLibrary.Array_Clear` _rally_circle_array))))

(event `UpdateRally`
  ;[0.09549 0.2229 1 0.264] POI Hab/Rally
  ;;[1 1 1 0.081] Rally Circle
  (bind _outactors (`GameplayStatics.GetAllActorsOfClass` "/Game/Gameplay/RallyPoint/BP_SquadRallyPoint.BP_SquadRallyPoint_C"))
  (for _array_element _outactors
    (bind _returnvalue (`KismetArrayLibrary.Array_AddUnique` (`self.Rally Array`) _array_element))
    (if (!= _returnvalue -1)
      (bind _returnvalue_2 (`|SpawnActorFromClass` "/CasterTools_Project/Settings/GamePlay/POI_Events/Circles/BP_Rally_Circle.BP_Rally_Circle_C" (`KismetMathLibrary.MakeTransform` (`SceneComponent.K2_GetComponentLocation` (`Actor.RootComponent` (`|GetArrayItem` (`self.Rally Array`) _returnvalue)))) "Undefined" "OverrideRootScale" null _array_element (`SQTeamState.Id` (`SQPlayerState.TeamState` (cast `SQPlayerState` (`self.PlayerState`) :!pure true))) null))
      (`KismetArrayLibrary.Array_Add` (`self.Rally Circle Array`) _returnvalue_2))))

(fn `ActorSpherePick`
  (bind _firstpersoncameracomponent (`self.FirstPersonCameraComponent`))
  (bind _current_target_actor (`self.Current Target Actor`))
  (bind _current_target_actor_2 (`self.Current Target Actor`))
  (bind _returnvalue (`SceneComponent.K2_GetComponentLocation` _firstpersoncameracomponent))
  (bind _returnvalue_2 (`KismetMathLibrary.Conv_RotatorToVector` (`SceneComponent.K2_GetComponentRotation` _firstpersoncameracomponent)))
  ;[1 1 1 0.394] Making Trace for Crosshair
  (bind _outhit (`KismetSystemLibrary.SphereTraceSingleForObjects` :`Start` (+ _returnvalue (* _returnvalue_2 (`KismetMathLibrary.Conv_DoubleToVector` 200.0))) :`End` (+ _returnvalue (* _returnvalue_2 (`KismetMathLibrary.Conv_DoubleToVector` (`self.Target Attachment Trace Dist`)))) :`ObjectTypes` (`|MakeArray` "ObjectTypeQuery3" "ObjectTypeQuery5" :!type "EObjectTypeQuery Enum") :`TraceColor` (struct :`R` 0.074214 :`G` 0.630757 :`B` 0.822786 :`A` 1.0)))
  (if (`KismetSystemLibrary.IsValid` (`.HitActor` (`GameplayStatics.BreakHitResult` _outhit)))
    (if (and (== _current_target_actor (`.HitActor` (`GameplayStatics.BreakHitResult` _outhit))) (`KismetSystemLibrary.IsValid` _current_target_actor))
      (`self.UpdateStensil`)
      (else
        (bind _output_get (set `self.Current Target Actor` (`.HitActor` (`GameplayStatics.BreakHitResult` _outhit))))
        (if (`KismetMathLibrary.ClassIsChildOf` (`GameplayStatics.GetObjectClass` _output_get) "/Script/Squad.SQSoldier")
          ;[1 1 1 0.217] Creating Outlines for Vic and Soldier
          (bind _asbp_mutable_soldier (cast `/Game/Blueprints/Soldiers/BP_MutableSoldier` _current_target_actor_2))
          (bind (_assqsoldier _bsuccess) (cast `SQSoldier` (`.HitActor` (`GameplayStatics.BreakHitResult` _outhit)) :!pure true))
          (if (or (and (not (`SQSoldier.bIsDying` _assqsoldier)) (not (`SQSoldier.bIsWounded` _assqsoldier)) (not (`Actor.bHidden` _assqsoldier))) (not _bsuccess))
            (bind _output_get_2 (set `self.As BP Mutable Soldier` _asbp_mutable_soldier))
            (`PrimitiveComponent.SetCustomDepthStencilValue` (`Character.Mesh` _output_get_2) 252))
          (else
            (bind _assqvehicle (cast `SQVehicle` _current_target_actor_2))
            (bind _output_get_3 (set `self.As SQVehicle` _assqvehicle))
            (bind _vehiclemesh (`SQVehicle.VehicleMesh` _output_get_3))
            (`PrimitiveComponent.SetRenderCustomDepth` _vehiclemesh true)
            (`PrimitiveComponent.SetCustomDepthStencilValue` _vehiclemesh 252)))))
    (else
      (`self.Current Target Actor`
        (:`then`
          (set `self.Current Target Actor` null)
          (bind _as_sqvehicle (`self.As SQVehicle`)
            (:`then`
              (`PrimitiveComponent.SetRenderCustomDepth` (`SQVehicle.VehicleMesh` _as_sqvehicle) false))
            (:`else`
              _)))
        (:`else`
          _))
      (set `self.As SQVehicle` null)
      (set `self.As BP Mutable Soldier` null))))

(fn `Attach POV Cam`
  (bind _w_infantry_status_caster (`self.W Infantry Status Caster`))
  (bind _cameraplayer (`self.CameraPlayer`))
  (bind _w_vehicle_status_caster (`self.W Vehicle Status Caster`))
  (bind _w_vehicle_status_caster_2 (`self.W Vehicle Status Caster`))
  (bind _springarm (`/CasterTools_Project/Settings/GamePlay/SpectateCam/BP_SpectateCam_Caster_M.SpringArm` (`self.CameraPlayer`)))
  (`|ExecutionSequence`
    (:`then_0`
      ;[1 1 1 0.245] Adding POV camera to Soldier
      (bind _as_bp_mutable_soldier (`self.As BP Mutable Soldier`)
        (:`then`
          (`|ExecutionSequence`
            (:`then_0`
              (`/CasterTools_Project/Settings/UI/CasterOverlay/Indicators/W_FollowName.GetSoldier DisplayName` (`self.W Follow Name`) _as_bp_mutable_soldier))
            (:`then_1`
              (`SceneComponent.K2_AttachToComponent` _springarm (`Character.Mesh` _as_bp_mutable_soldier) (`self.Socket Name`) "SnapToTarget" "SnapToTarget" "KeepRelative" true)
              (`SceneComponent.K2_AddLocalOffset` _springarm (10.0 -14.0 0.0) false true)
              (`SceneComponent.K2_SetRelativeRotation` _springarm (`KismetMathLibrary.MakeRotator` 0.0 6.0 -60.0) false false)
              (`Widget.SetVisibility` (`self.SpectatorCamWidget`) "Visible")
              (set `/CasterTools_Project/Settings/UI/CasterOverlay/Indicators/Infantry_Status/W_InfantryStatusCaster.MutableSoldier` (`self.As BP Mutable Soldier`) _w_infantry_status_caster)
              (`Widget.SetVisibility` _w_infantry_status_caster "Visible")
              (`/CasterTools_Project/Settings/UI/CasterOverlay/Indicators/Infantry_Status/W_InfantryStatusCaster.Entered` _w_infantry_status_caster)
              (`Widget.SetVisibility` (`self.W Follow Name`) "Visible"))))
        (:`else`)))
    (:`then_1`
      ;[1 1 1 0.258] Vehicle Cam Logic
      (bind _as_sqvehicle (`self.As SQVehicle`)
        (:`then`
          (`|ExecutionSequence`
            (:`then_0`
              (bind _returnvalue (`SQVehicleSeatComponent.GetSeatPawn` (`|GetArrayItem` (`SQVehicle.GetSeats` _as_sqvehicle) 1)))
              (`/Engine/EditorBlueprintResources/StandardMacros.IsValid` _returnvalue
                (:`Is Valid`
                  (bind _assqvehicle_turret_closed_top (cast `SQVehicleTurretClosedTop` _returnvalue)
                    (:`then`
                      (`SceneComponent.K2_AttachToComponent` (`/CasterTools_Project/Settings/GamePlay/SpectateCam/BP_SpectateCam_Caster_M.SpringArm` _cameraplayer) (`SQVehicleSeat.GetCameraComponent` _assqvehicle_turret_closed_top) "None" "SnapToTarget" "SnapToTarget" "SnapToTarget" true)
                      (set `SceneCaptureComponent2D.FOVAngle` 66.0 (`/CasterTools_Project/Settings/GamePlay/SpectateCam/BP_SpectateCam_Caster_M.SceneCaptureComponent2D` _cameraplayer))
                      (`Widget.SetVisibility` (`self.SpectatorCamWidget`) "HitTestInvisible")
                      (`Widget.SetVisibility` (`self.W Follow Name`) "HitTestInvisible")
                      (`Widget.SetVisibility` _w_vehicle_status_caster_2 "HitTestInvisible")
                      (set `/CasterTools_Project/Settings/UI/CasterOverlay/Indicators/Vehicle_Status/W_VehicleStatusCaster.Vehicle_Ref` _as_sqvehicle _w_vehicle_status_caster_2)
                      (`/CasterTools_Project/Settings/UI/CasterOverlay/Indicators/Vehicle_Status/W_VehicleStatusCaster.GetVicIcon` _w_vehicle_status_caster_2))
                    (:`CastFailed`
                      ;;[1 0.03963 0.09936 0.426] Vics without Turret
                      (`Widget.SetVisibility` (`self.W Follow Name`) "HitTestInvisible" :!label _label)
                      (`Widget.SetVisibility` _w_vehicle_status_caster "HitTestInvisible")
                      (set `/CasterTools_Project/Settings/UI/CasterOverlay/Indicators/Vehicle_Status/W_VehicleStatusCaster.Vehicle_Ref` _as_sqvehicle _w_vehicle_status_caster)
                      (`/CasterTools_Project/Settings/UI/CasterOverlay/Indicators/Vehicle_Status/W_VehicleStatusCaster.GetVicIcon` _w_vehicle_status_caster))))
                (:`Is Not Valid`
                  (goto _label))))
            (:`then_1`
              (`/CasterTools_Project/Settings/UI/CasterOverlay/Indicators/W_FollowName.Get VehicleName` (`self.W Follow Name`) _as_sqvehicle))))
        (:`else`)))))

(fn `Dettach POV Cam`
  (bind _cameraplayer (`self.CameraPlayer`))
  (bind _springarm (`/CasterTools_Project/Settings/GamePlay/SpectateCam/BP_SpectateCam_Caster_M.SpringArm` _cameraplayer))
  (`SceneComponent.K2_AddLocalOffset` _springarm (0.0 0.0 0.0) false true)
  (set `SceneCaptureComponent2D.FOVAngle` 90.0 (`/CasterTools_Project/Settings/GamePlay/SpectateCam/BP_SpectateCam_Caster_M.SceneCaptureComponent2D` _cameraplayer))
  (`Widget.SetVisibility` (`self.SpectatorCamWidget`) "Collapsed")
  (`Widget.SetVisibility` (`self.W Infantry Status Caster`) "Collapsed")
  (`Widget.SetVisibility` (`self.W Vehicle Status Caster`) "Collapsed")
  (`Widget.SetVisibility` (`self.W Follow Name`) "Collapsed")
  (`SceneComponent.K2_DetachFromComponent` _springarm "KeepRelative" "KeepRelative" "KeepRelative" true))

(fn `DettachFollowCam`
  (`self.DetachAdminCamFromActor` (`self.DefaultMovementMode`)))

(fn `Enter Follow Cam`
  (locals (L_SkeletalMesh :type "SkeletalMeshComponent Object Reference"))
  (bind _followoffsetdistancethreshold_x (`KismetMathLibrary.BreakVector2D` (`self.FollowOffsetDistanceThreshold`)))
  (if (not (`self.bIsFollowingActor`))
    (`self.ExitFollowCam`))
  (bind _current_target_actor (`self.Current Target Actor`)
    (:`then`
      (bind _output_get (set `self.CurrentFollowTarget` _current_target_actor))
      (set `self.Current Target Actor` null)
      (bind _assqsoldier (cast `SQSoldier` _output_get)
        (:`then`
          (set `local.L_SkeletalMesh` (`Character.Mesh` _assqsoldier))
          (if (and (not (`SQSoldier.bIsWounded` _assqsoldier)) (not (`SQSoldier.bIsDying` _assqsoldier)))
            (add `SQSoldier.OnWoundEvent` _assqsoldier (`|CreateDelegate` :!event `OnFollowedPlayerWounded`))
            (add `SQSoldier.OnDeathEvent` _assqsoldier (`|CreateDelegate` :!event `OnFollowSoldierDeath`))
            (set `self.OptionalFollowOffsetHeight` -320.0)
            (bind (_returnvalue_x _returnvalue_y _returnvalue_z) (`KismetMathLibrary.BreakVector` (/ (`.BoxExtent` (`self.GetActorBounds` _output_get true false)) (2.0 2.0 2.0))))
            (bind _output_get_2 (set `self.BaseFollowOffsetDistance` (+ (* _returnvalue_x -1.0) (* _followoffsetdistancethreshold_x -1.0)) :!label _label))
            (set `self.FollowOffset` (`KismetMathLibrary.MakeVector` _output_get_2 0.0 (+ (`self.OptionalFollowOffsetHeight`) (+ _returnvalue_z (`self.BaseFollowOffsetHeight`)))))
            (add `self.OnDestroyed` _output_get (`|CreateDelegate` :!event `OnFollowTargetDestroyed`))
            (add `self.OnEndPlay` _output_get (`|CreateDelegate` :!event `OnFollowTargetEndPlay`))
            (`self.Attach FollowCam` _output_get (`local.L_SkeletalMesh`))))
        (:`CastFailed`
          (bind _assqvehicle (cast `SQVehicle` _output_get))
          (set `local.L_SkeletalMesh` (`SQVehicle.VehicleMesh` _assqvehicle))
          (add `SQVehicle.OnVehicleDestroyed` _assqvehicle (`|CreateDelegate` :!event `OnFollowVehicleDestroyed`))
          (set `self.OptionalFollowOffsetHeight` 0.0)
          (goto _label))))
    (:`else`)))

(fn `ExitFollowCam`
  (bind _currentfollowtarget (`self.CurrentFollowTarget`))
  (bind _currentfollowtarget_2 (`self.CurrentFollowTarget`))
  (bind _assqsoldier (cast `SQSoldier` _currentfollowtarget_2)
    (:`then`
      (remove `SQSoldier.OnDeathEvent` _assqsoldier (`|CreateDelegate` :!event `OnFollowSoldierDeath`))
      (remove `SQSoldier.OnWoundEvent` (cast `/Game/Blueprints/Soldiers/BP_MutableSoldier` _assqsoldier :!pure true) (`|CreateDelegate` :!event `OnFollowedPlayerWounded`)))
    (:`CastFailed`
      (bind _assqvehicle (cast `SQVehicle` _currentfollowtarget_2))
      (remove `SQVehicle.OnVehicleDestroyed` _assqvehicle (`|CreateDelegate` :!event `OnFollowVehicleDestroyed`))))
  (remove `self.OnDestroyed` _currentfollowtarget (`|CreateDelegate` :!event `OnFollowTargetDestroyed`))
  (remove `self.OnEndPlay` _currentfollowtarget (`|CreateDelegate` :!event `OnFollowTargetEndPlay`))
  (`self.DettachFollowCam`)
  (set `self.CurrentFollowTarget` null)
  (set `self.bIsFollowingActor` false))

(fn `UpdateStensil`
  (`|ExecutionSequence`
    (:`then_0`
      (bind _as_bp_mutable_soldier (`self.As BP Mutable Soldier`)
        (:`then`
          (`PrimitiveComponent.SetCustomDepthStencilValue` (`Character.Mesh` _as_bp_mutable_soldier) 252))
        (:`else`)))
    (:`then_1`
      (bind _as_sqvehicle (`self.As SQVehicle`)
        (:`then`
          (`PrimitiveComponent.SetCustomDepthStencilValue` (`SQVehicle.VehicleMesh` _as_sqvehicle) 252))
        (:`else`)))))

(fn `UserConstructionScript`
  (`parent.UserConstructionScript`))